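; StickBox is a trigger volume that flags the first-person character as touching a wall and halts its movement, apparently to make it stick.
; On Box overlap, it sets the character's IsTouchingWall to true, then stops its movement immediately after a short delay.
; Ending the overlap clears the flag but does not cancel a pending delayed stop.
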(event `self.Box.OnComponentBeginOverlap`
  (params (OverlappedComponent :type "PrimitiveComponent Object Reference") (OtherActor :type "Actor Object Reference") (OtherComp :type "PrimitiveComponent Object Reference") (OtherBodyIndex :type Integer) (bFromSweep :type Boolean) (SweepResult :type "HitResult Structure (by ref)"))
  (bind _firstpersonref (`self.FirstPersonRef`))
  (bind _asfirst_person_character (cast `/Game/FirstPersonBP/Blueprints/FirstPersonCharacter` OtherActor))
  (bind _output_get (set `self.FirstPersonRef` _asfirst_person_character))
  (set `/Game/FirstPersonBP/Blueprints/FirstPersonCharacter.IsTouchingWall?` true _firstpersonref)
  (`KismetSystemLibrary.Delay` 0.5)
  (`MovementComponent.StopMovementImmediately` (`Character.CharacterMovement` _firstpersonref)))

(event `self.Box.OnComponentEndOverlap`
  (params (OverlappedComponent :type "PrimitiveComponent Object Reference") (OtherActor :type "Actor Object Reference") (OtherComp :type "PrimitiveComponent Object Reference") (OtherBodyIndex :type Integer))
  (bind _asfirst_person_character (cast `/Game/FirstPersonBP/Blueprints/FirstPersonCharacter` OtherActor))
  (bind _output_get (set `self.FirstPersonRef` _asfirst_person_character))
  (set `/Game/FirstPersonBP/Blueprints/FirstPersonCharacter.IsTouchingWall?` false (`self.FirstPersonRef`)))

(fn `UserConstructionScript`)